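; Enemy NPC character that can be fought or killed by stealth assassination, with a health bar.
; Damage plays a random hit montage, launches it along the player's facing and feeds BPCPlayerStats; death ragdolls it and notifies the player's quest component.
; An overlap radius shows a camera-facing assassination prompt for the player.
; StealthBackAssassin plays the victim montage, triggers delayed ragdoll and returns attacker alignment, without notifying the quest.
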(event `self.ReceiveBeginPlay`
  (bind _aswb_enemy_hud (cast `/Game/UI/WB_EnemyHUD` (`WidgetComponent.GetWidget` (`self.HealthBar`))))
  (set `self.HealthBarUI(Enemy)` _aswb_enemy_hud))

(event `self.ReceiveTick`
  (params (DeltaSeconds :type "Float (single-precision)"))
  (`SceneComponent.K2_SetWorldRotation` (`self.AssassinateWidget`) (`KismetMathLibrary.FindLookAtRotation` (`SceneComponent.K2_GetComponentLocation` (`self.AssassinateWidget`)) (`SceneComponent.K2_GetComponentLocation` (`PlayerCameraManager.TransformComponent` (`GameplayStatics.GetPlayerCameraManager` 0)))) false false))

(event `Ragdoll`
  ;[0.01938 0.01938 0.01938] Ragdoll
  (`KismetSystemLibrary.Delay` 2.5)
  (`PrimitiveComponent.SetSimulatePhysics` (`self.Mesh`) true))

(event `self.AssassinationRadius.OnComponentBeginOverlap`
  (params (OverlappedComponent :type "PrimitiveComponent Object Reference") (OtherActor :type "Actor Object Reference") (OtherComp :type "PrimitiveComponent Object Reference") (OtherBodyIndex :type Integer) (bFromSweep :type Boolean) (SweepResult :type "HitResult Structure (by ref)"))
  (cast `/Game/ThirdPerson/Blueprints/BP_ThirdPersonCharacter` OtherActor)
  (`SceneComponent.SetVisibility` (`self.AssassinateWidget`) true false))

(event `self.AssassinationRadius.OnComponentEndOverlap`
  (params (OverlappedComponent :type "PrimitiveComponent Object Reference") (OtherActor :type "Actor Object Reference") (OtherComp :type "PrimitiveComponent Object Reference") (OtherBodyIndex :type Integer))
  (cast `/Game/ThirdPerson/Blueprints/BP_ThirdPersonCharacter` OtherActor)
  (`SceneComponent.SetVisibility` (`self.AssassinateWidget`) false false))

(event `self.ReceiveAnyDamage`
  (params (Damage :type "Float (single-precision)") (DamageType :type "DamageType Object Reference") (InstigatedBy :type "Controller Object Reference") (DamageCauser :type "Actor Object Reference"))
  ;[0.05127 0.05127 0.05127] Take Damage Ai
  (`self.PlayAnimMontage` (`|GetArrayItem` (`self.Hit_Anim`) (`KismetMathLibrary.RandomIntegerInRange` 0 (- (`KismetArrayLibrary.Array_Length` (`self.Hit_Anim`)) 1))))
  (bind _asbp_third_person_character (cast `/Game/ThirdPerson/Blueprints/BP_ThirdPersonCharacter` (`GameplayStatics.GetPlayerCharacter` 0)))
  (`self.LaunchCharacter` (* (`KismetMathLibrary.GetForwardVector` (`self.K2_GetActorRotation` _asbp_third_person_character)) 700.0))
  (bind _playerdead_ (`/Game/AI/Blueprint/BPC_PlayerStats.Decrease Health` (`self.BPC_PlayerStats`) Damage))
  (if _playerdead_
    (`PrimitiveComponent.SetCollisionObjectType` (`self.Mesh`) "ECC_PhysicsBody")
    (`PrimitiveComponent.SetSimulatePhysics` (`self.Mesh`) true)
    (`SceneComponent.SetVisibility` (`self.HealthBar`) false false)
    (`CharacterMovementComponent.SetMovementMode` (`self.CharacterMovement`) "MOVE_None" 0)
    (bind _asbp_third_person_character_2 (cast `/Game/ThirdPerson/Blueprints/BP_ThirdPersonCharacter` (`GameplayStatics.GetPlayerCharacter` 0)))
    (`/Game/ThirdPerson/Blueprints/BPC_Quest.Eliminate Enemies` (`/Game/ThirdPerson/Blueprints/BP_ThirdPersonCharacter.BPC_Quest` _asbp_third_person_character_2) self)))

(fn `StealthBackAssassin`
  (returns (RefLocation :type "Vector Structure") (AssassinRotation :type "Rotator Structure"))
  (`self.PlayAnimMontage` "/Game/Animations/Assassination/Paired_Knife_Stealth_KidneyAndNeck_Vic_Montage.Paired_Knife_Stealth_KidneyAndNeck_Vic_Montage")
  (`self.Ragdoll`)
  (`SceneComponent.SetVisibility` (`self.AssassinateWidget`) false false)
  (`SceneComponent.SetVisibility` (`self.HealthBar`) false false)
  (`CharacterMovementComponent.SetMovementMode` (`self.CharacterMovement`) "MOVE_None" 0)
  (return (`SceneComponent.K2_GetComponentLocation` (`self.AssassinationRef`)) (`self.K2_GetActorRotation`)))

(fn `UserConstructionScript`)