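; Stats component that tracks health and stamina for the player character, and is also used on BP_Enemy for health.
; On BeginPlay it waits a tick, casts its owner to set IsPlayer, and initializes the HUD or enemy health bar.
; Decrease functions return true on depletion, while increase functions raise maximums or clamp restored values.
; Each updates UI directly, but only DecreaseHealth supports the enemy bar.
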(event `self.ReceiveBeginPlay`
  (`KismetSystemLibrary.DelayUntilNextTick`)
  (bind _asbp_third_person_character (cast `/Game/ThirdPerson/Blueprints/BP_ThirdPersonCharacter` (`self.GetOwner`))
    (:`then`
      (set `self.PlayerCharacterBP` _asbp_third_person_character)
      (set `self.isPlayer` true)
      (`ProgressBar.SetPercent` (`/Game/UI/WBC_HUD.Stamina` (`/Game/ThirdPerson/Blueprints/BP_ThirdPersonCharacter.HUD Widget` (`self.PlayerCharacterBP`))) (/ (`self.CurrentStamina`) (`self.MaxStamina`)))
      (`TextBlock.SetText` (select `bool` (`self.isPlayer`) :`false` (`/Game/UI/WB_EnemyHUD.HealthText` (`/Game/AI/Blueprint/BP_Enemy.HealthBarUI(Enemy)` (`self.BP_Enemy`))) :`true` (`/Game/UI/WBC_HUD.HealthText` (`/Game/ThirdPerson/Blueprints/BP_ThirdPersonCharacter.HUD Widget` (`self.PlayerCharacterBP`)))) (`KismetTextLibrary.Conv_DoubleToText` (`self.CurrentHealth`) "HalfToEven")))
    (:`CastFailed`
      (bind _asbp_enemy (cast `/Game/AI/Blueprint/BP_Enemy` (`self.GetOwner`)))
      (set `self.BP_Enemy` _asbp_enemy)
      (set `self.isPlayer` false)))
  (`ProgressBar.SetPercent` (select `bool` (`self.isPlayer`) :`false` (`/Game/UI/WB_EnemyHUD.Health` (`/Game/AI/Blueprint/BP_Enemy.HealthBarUI(Enemy)` (`self.BP_Enemy`))) :`true` (`/Game/UI/WBC_HUD.Health` (`/Game/ThirdPerson/Blueprints/BP_ThirdPersonCharacter.HUD Widget` (`self.PlayerCharacterBP`)))) (/ (`self.CurrentHealth`) (`self.MaxHealth`))))

(fn `Decrease Health`
  (params (Damage :type "Float (double-precision)"))
  (returns (`playerDead?` :type Boolean))
  (if (not (<= (`self.CurrentHealth`) 0.0))
    (bind _output_get (set `self.CurrentHealth` (- (`self.CurrentHealth`) Damage)))
    (`ProgressBar.SetPercent` (select `bool` (`self.isPlayer`) :`false` (`/Game/UI/WB_EnemyHUD.Health` (`/Game/AI/Blueprint/BP_Enemy.HealthBarUI(Enemy)` (`self.BP_Enemy`))) :`true` (`/Game/UI/WBC_HUD.Health` (`/Game/ThirdPerson/Blueprints/BP_ThirdPersonCharacter.HUD Widget` (`self.PlayerCharacterBP`)))) (/ _output_get (`self.MaxHealth`)))
    (`TextBlock.SetText` (select `bool` (`self.isPlayer`) :`false` (`/Game/UI/WB_EnemyHUD.HealthText` (`/Game/AI/Blueprint/BP_Enemy.HealthBarUI(Enemy)` (`self.BP_Enemy`))) :`true` (`/Game/UI/WBC_HUD.HealthText` (`/Game/ThirdPerson/Blueprints/BP_ThirdPersonCharacter.HUD Widget` (`self.PlayerCharacterBP`)))) (`KismetTextLibrary.Conv_DoubleToText` (`self.CurrentHealth`) "HalfToEven"))
    (if (<= (`self.CurrentHealth`) 0.0)
      _
      (else
        (return false))))
  (return true))

(fn `DecreaseStamina`
  (params (StaminaDepleted :type "Float (double-precision)"))
  (returns (`NoStaminaLeft?` :type Boolean))
  (if (not (<= (`self.CurrentStamina`) 0.0))
    (set `self.CurrentStamina` (- (`self.CurrentStamina`) StaminaDepleted))
    (`ProgressBar.SetPercent` (`/Game/UI/WBC_HUD.Stamina` (`/Game/ThirdPerson/Blueprints/BP_ThirdPersonCharacter.HUD Widget` (`self.PlayerCharacterBP`))) (/ (`self.CurrentStamina`) (`self.MaxStamina`)))
    (if (<= (`self.CurrentStamina`) 0.0)
      _
      (else
        (return false))))
  (return true))

(fn `IncreaseHealth`
  (params (`Added Health` :type "Float (double-precision)"))
  (bind _hud_widget (`/Game/ThirdPerson/Blueprints/BP_ThirdPersonCharacter.HUD Widget` (`self.PlayerCharacterBP`)))
  (set `self.CurrentHealth` (+ (`self.CurrentHealth`) `Added Health`))
  (if (> (`self.CurrentHealth`) (`self.MaxHealth`))
    (set `self.CurrentHealth` (`self.MaxHealth`)))
  (`ProgressBar.SetPercent` (`/Game/UI/WBC_HUD.Health` _hud_widget) (/ (`self.CurrentHealth`) (`self.MaxHealth`)))
  (`TextBlock.SetText` (`/Game/UI/WBC_HUD.HealthText` _hud_widget) (`KismetTextLibrary.Conv_DoubleToText` (`self.CurrentHealth`) "HalfToEven")))

(fn `IncreaseMaxHealth`
  (params (IncreaseHealth :type "Float (double-precision)"))
  (bind _hud_widget (`/Game/ThirdPerson/Blueprints/BP_ThirdPersonCharacter.HUD Widget` (`self.PlayerCharacterBP`)))
  (set `self.MaxHealth` (+ (`self.MaxHealth`) IncreaseHealth))
  (`ProgressBar.SetPercent` (`/Game/UI/WBC_HUD.Health` _hud_widget) (/ (`self.CurrentHealth`) (`self.MaxHealth`)))
  (`TextBlock.SetText` (`/Game/UI/WBC_HUD.HealthText` _hud_widget) (`KismetTextLibrary.Conv_DoubleToText` (`self.CurrentHealth`) "HalfToEven")))

(fn `IncreaseMaxStamina`
  (params (IncreaseStamina :type "Float (double-precision)"))
  (set `self.MaxStamina` (+ (`self.MaxStamina`) IncreaseStamina))
  (`ProgressBar.SetPercent` (`/Game/UI/WBC_HUD.Stamina` (`/Game/ThirdPerson/Blueprints/BP_ThirdPersonCharacter.HUD Widget` (`self.PlayerCharacterBP`))) (/ (`self.CurrentStamina`) (`self.MaxStamina`))))

(fn `IncreaseStamina`
  (params (`Added Stamina` :type "Float (double-precision)"))
  (set `self.CurrentStamina` (+ (`self.CurrentStamina`) `Added Stamina`))
  (if (> (`self.CurrentStamina`) (`self.MaxStamina`))
    (set `self.CurrentStamina` (`self.MaxStamina`)))
  (`ProgressBar.SetPercent` (`/Game/UI/WBC_HUD.Stamina` (`/Game/ThirdPerson/Blueprints/BP_ThirdPersonCharacter.HUD Widget` (`self.PlayerCharacterBP`))) (/ (`self.CurrentStamina`) (`self.MaxStamina`))))