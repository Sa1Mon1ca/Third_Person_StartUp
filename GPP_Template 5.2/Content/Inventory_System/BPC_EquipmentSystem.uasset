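; Equipment component for the third-person character that handles weapon pickup and the equipment menu.
; The pickup input sphere-traces from the follow camera, appends a hit weapon's item data to the weapon slot array and destroys that actor.
; The inventory input toggles a lazily created, reused equipment widget, switching cursor and input mode while disabling attacks and movement as the panel is open.
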(event `self.ReceiveBeginPlay`
  (bind _asbp_third_person_character (cast `/Game/ThirdPerson/Blueprints/BP_ThirdPersonCharacter` (`self.GetOwner`)))
  (set `self.Follow Camera` (`/Game/ThirdPerson/Blueprints/BP_ThirdPersonCharacter.FollowCamera` _asbp_third_person_character))
  (set `self.BPC Attack Class` (`/Game/ThirdPerson/Blueprints/BP_ThirdPersonCharacter.BPC_AttackClass` _asbp_third_person_character)))

(event `EnhancedInput|/Game/ThirdPerson/Input/Actions/IA_Pickup`
  (params (ActionValue :type Boolean) (ElapsedSeconds :type "Float (double-precision)") (TriggeredSeconds :type "Float (double-precision)") (InputAction :type "InputAction Object Reference" :default "/Game/ThirdPerson/Input/Actions/IA_Pickup.IA_Pickup"))
  (bind _follow_camera (`self.Follow Camera`))
  (bind _returnvalue (`SceneComponent.K2_GetComponentLocation` _follow_camera))
  ;[0.05127 0.05127 0.05127] Pickup Trace
  (:`Started`
    (bind (_outhit _returnvalue_2) (`KismetSystemLibrary.SphereTraceSingleForObjects` _returnvalue (+ _returnvalue (* (`KismetMathLibrary.GetForwardVector` (`SceneComponent.K2_GetComponentRotation` _follow_camera)) 1000.0)) 15.0 (`|MakeArray` "ObjectTypeQuery2" :!type "EObjectTypeQuery Enum")))
    (if _returnvalue_2
      (bind _asbp_weapon (cast `/Game/Inventory_System/BP_Weapon` (`.HitActor` (`GameplayStatics.BreakHitResult` _outhit))))
      (`self.Add_Weapon` (`/Game/Inventory_System/BP_Weapon.itemData` _asbp_weapon))
      (`Actor.K2_DestroyActor` _asbp_weapon))))

(event `EnhancedInput|/Game/ThirdPerson/Input/Actions/IA_OpenInventory`
  (params (ActionValue :type Boolean) (ElapsedSeconds :type "Float (double-precision)") (TriggeredSeconds :type "Float (double-precision)") (InputAction :type "InputAction Object Reference" :default "/Game/ThirdPerson/Input/Actions/IA_OpenInventory.IA_OpenInventory"))
  (bind _returnvalue (`GameplayStatics.GetPlayerController` 0))
  (bind _bpc_attack_class (`self.BPC Attack Class`))
  ;[0.05127 0.05127 0.05127] Equipment Menu Panel
  (:`Started`
    (if (not (`self.isPanelOpen?`))
      (set `/Game/ThirdPerson/Blueprints/BPC_AttackClass.can Attack?` false _bpc_attack_class)
      (set `self.isPanelOpen?` true)
      (bind _equipmentwidget (`self.EquipmentWidget`)
        (:`then`
          (`Widget.SetVisibility` _equipmentwidget "Visible"))
        (:`else`
          (bind _returnvalue_2 (`|CreateWidget` "/Game/Inventory_System/UI/WB_Equipment.WB_Equipment_C"))
          (bind _output_get (set `self.EquipmentWidget` _returnvalue_2))
          (`UserWidget.AddToViewport` _output_get 0)))
      (set `PlayerController.bShowMouseCursor` true _returnvalue)
      (`WidgetBlueprintLibrary.SetInputMode_GameAndUIEx` _returnvalue (`self.EquipmentWidget`))
      (bind _asbp_third_person_character (cast `/Game/ThirdPerson/Blueprints/BP_ThirdPersonCharacter` (`self.GetOwner`)))
      (`CharacterMovementComponent.SetMovementMode` (`Character.CharacterMovement` _asbp_third_person_character) "MOVE_None" 0)
      (else
        (set `/Game/ThirdPerson/Blueprints/BPC_AttackClass.can Attack?` true _bpc_attack_class)
        (set `self.isPanelOpen?` false)
        (bind _equipmentwidget_2 (`self.EquipmentWidget`)
          (:`then`
            (`Widget.SetVisibility` _equipmentwidget_2 "Hidden")
            (set `PlayerController.bShowMouseCursor` false _returnvalue)
            (`WidgetBlueprintLibrary.SetInputMode_GameOnly` _returnvalue)
            (bind _asbp_third_person_character_2 (cast `/Game/ThirdPerson/Blueprints/BP_ThirdPersonCharacter` (`self.GetOwner`)))
            (`CharacterMovementComponent.SetMovementMode` (`Character.CharacterMovement` _asbp_third_person_character_2) "MOVE_Walking" 0))
          (:`else`))))))

(fn `Add_Weapon`
  (params (NewItem :type "/Game/Inventory_System/S_Slot Structure (by ref)"))
  (`KismetArrayLibrary.Array_Add` (`self.Weapon_Slot`) NewItem))